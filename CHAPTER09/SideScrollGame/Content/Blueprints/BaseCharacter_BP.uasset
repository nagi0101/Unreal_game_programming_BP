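; BaseCharacter_BP is a base character Blueprint that gives an actor health, death and a score value.
; Construction sets Health to HealthMax, and AnyDamage subtracts incoming damage from it.
; The death check subtracts Damage again from the updated Health, so death triggers one hit's worth early.
; DeathEvent spawns the death effect, adds KillScore through the MyGame game mode, then destroys the actor.
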(event EventBeginPlay)

(event Collision|EventActorBeginOverlap
  (params (OtherActor :type Actor%20Object%20Reference)))

(event EventTick
  (params (DeltaSeconds :type Float%20%28single-precision%29)))

(event Game|Damage|EventAnyDamage
  (params (Damage :type Float%20%28single-precision%29) (DamageType :type Damage%20Type%20Object%20Reference) (InstigatedBy :type Controller%20Object%20Reference) (DamageCauser :type Actor%20Object%20Reference))
  (Variables|Default|SetHealth (- (Variables|Default|GetHealth) Damage))
  (if (> 0.0 (- (Variables|Default|GetHealth) Damage))
    (CallFunction|DeathEvent)))

(fn ConstructionScript
  (Variables|Default|SetHealth (Variables|Default|GetHealthMax)))

(fn DeathEvent
  (Effects|SpawnEmitteratLocation (Variables|Default|GetDeathEffect) (Transformation|GetActorLocation))
  (bind _asmy_game (Utilities|Casting|CastToMyGame (Game|GetGameMode)))
  (Default|AddScore _asmy_game (Variables|Default|GetKillScore))
  (Actor|DestroyActor))