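; HUD Blueprint that draws health bars and score labels on the canvas each frame.
; BeginPlay caches the MyGame game mode and the owning pawn as MyCharacter.
; DrawHUD draws a player health bar and projects every MyEnemy location to screen space for health-sized bars, finding enemies with GetAllActorsOfClass every draw.
; The center text and both Score and High Score labels use the game mode's display name.
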(event EventBeginPlay
  (bind _asmy_game (Utilities|Casting|CastToMyGame (Variables|Default|GetGameMode)))
  (Variables|Default|SetGameMode _asmy_game)
  (bind _asmy_character (Utilities|Casting|CastToMyCharacter (Class|HUD|GetOwningPawn)))
  (Variables|Default|SetCharacter _asmy_character))

(event Collision|EventActorBeginOverlap
  (params (OtherActor :type Actor%20Object%20Reference)))

(event EventTick
  (params (DeltaSeconds :type Float%20%28single-precision%29)))

(event EventDrawHUD
  (params (SizeX :type Integer) (SizeY :type Integer))
  (bind _gamemode (Variables|Default|GetGameMode))
  (bind _textcolor (Variables|Default|GetTextColor))
  (HUD|DrawText (Utilities|GetDisplayName (Variables|Default|GetGameMode)) (Variables|Default|GetTextColor) (* (Math|Conversions|ToFloat(Integer) SizeX) 0.5) (* (Math|Conversions|ToFloat(Integer) SizeY) 0.5) 0 1.0 false)
  (Utilities|FlowControl|Sequence
    (:then_0
      (HUD|DrawRect (Variables|Default|GetTextColor) 0.0 0.0 (* (Variables|/Game/Blueprints/BaseCharacter_BP.BaseCharacter_BP_C|GetHealth (Variables|Default|GetCharacter)) 2.0) 0.0))
    (:then_1
      (bind _outactors (Actor|GetAllActorsOfClass "/Game/Blueprints/MyEnemy.MyEnemy_C"))
      (for _array_element _outactors
        (bind _asmy_enemy (Utilities|Casting|CastToMyEnemy _array_element))
        (HUD|DrawRect (Variables|Default|GetTextColor) (.X (Math|Vector|BreakVector (Class|HUD|Project (Transformation|GetActorLocation _asmy_enemy)))) (.Y (Math|Vector|BreakVector (Class|HUD|Project (Transformation|GetActorLocation _asmy_enemy)))) (Variables|/Game/Blueprints/BaseCharacter_BP.BaseCharacter_BP_C|GetHealth _asmy_enemy) 0.0)))
    (:then_2
      (HUD|DrawText (Utilities|String|Append "Score" (Utilities|GetDisplayName _gamemode)) _textcolor 0.0 0.0 0 1.0 false))
    (:then_3
      (HUD|DrawText (Utilities|String|Append "High Score" (Utilities|GetDisplayName _gamemode)) _textcolor 0.0 0.0 0 1.0 false))))

(fn ConstructionScript)